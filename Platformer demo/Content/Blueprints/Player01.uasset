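; Player character Blueprint with an advanced movement kit: run and crouch toggles, double jump, gliding, sliding and wall running with wall jumps.
; Q in mid-air sphere-traces both sides, then a looping timer drives Flying-mode movement along the wall normal's cross product until timeout or contact loss.
; Double and wall jumps bind the apex event, which lowers gravity and raises air control to glide.
; R slides by crouching with zero ground friction.
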(event `InputAction|CrouchKey`
  (params (Key :type "Key Structure"))
  ; Actions
  (:`Pressed`
    (`/Engine/EditorBlueprintResources/StandardMacros.FlipFlop`
      (:`A`
        (`self.Crouch`)
        (set `self.SpeedModifier` 0.3))
      (:`B`
        (`self.UnCrouch`)
        (set `self.SpeedModifier` 1.0)))))

(event `InputAction|Jump`
  (params (Key :type "Key Structure"))
  (bind _charactermovement (`self.CharacterMovement`))
  (bind _charactermovement_2 (`self.CharacterMovement`))
  (bind _jumpcount (`self.jumpcount`))
  (bind (_returnvalue_x _returnvalue_y) (`KismetMathLibrary.BreakVector` (+ (`self.GetActorForwardVector`) (* (`self.GetActorRightVector`) (* (`KismetMathLibrary.SelectFloat` 1.0 -1.0 (`|EnumEquality` (`self.wallslide`) "NewEnumerator0")) 800.0)))))
  ; For jump and double jump
  (:`Pressed`
    ; for wall jumping
    (if (`self.wallrunning`)
      (`|ExecutionSequence`
        (:`then_0`
          (`self.stopwallrun` "MOVE_Falling")
          (`|ExecutionSequence`
            (:`then_0`
              (`self.LaunchCharacter` (`KismetMathLibrary.MakeVector` _returnvalue_x _returnvalue_y 800.0))
              ;; For gliding
              (`|ExecutionSequence` :!label _label
                (:`then_0`
                  (`/Engine/EditorBlueprintResources/StandardMacros.IncrementInt` (`self.jumpcount`) :!label _label_2))
                (:`then_1`
                  (set `CharacterMovementComponent.bNotifyApex` true _charactermovement)
                  (add `self.OnReachedJumpApex` (`|CreateDelegate` :!event `OnApexReached`)))))
            (:`then_1`
              (set `self.jumpcount` 1)))))
      (elif (== _jumpcount 0)
        (`self.Jump`)
        (`KismetSystemLibrary.Delay` 0.2)
        (goto _label_2)
        (elif (< _jumpcount 2)
          (`self.LaunchCharacter` (0.0 0.0 600.0))
          (goto _label)))))
  (:`Released`
    (`self.StopJumping`)
    (set `CharacterMovementComponent.bNotifyApex` (== (`self.jumpcount`) 3) _charactermovement)
    (clear `self.OnReachedJumpApex`)
    (set `CharacterMovementComponent.GravityScale` 1.0 _charactermovement_2)
    (set `CharacterMovementComponent.AirControl` 0.05 _charactermovement_2)))

(event `InputAxis|moveforwardbackward`
  (params (AxisValue :type "Float (single-precision)"))
  ; Movement
  (`self.AddMovementInput` (`KismetMathLibrary.GetForwardVector` (`KismetMathLibrary.MakeRotator` 0.0 0.0 (.yaw (`self.GetControlRotation`)))) (* AxisValue (`self.SpeedModifier`)))
  (set `self.capsule radius` (`CapsuleComponent.GetUnscaledCapsuleRadius` (`self.CapsuleComponent`)) :!label _label_3) ; for wall running
)

(event `self.OnLanded`
  (params (Hit :type "HitResult Structure (by ref)"))
  (bind _charactermovement (`self.CharacterMovement`))
  ; For jump and double jump
  (`|ExecutionSequence`
    (:`then_0`
      (set `self.jumpcount` 0))
    (:`then_1`
      ;; For gliding
      (set `CharacterMovementComponent.GravityScale` 1.0 _charactermovement)
      (set `CharacterMovementComponent.AirControl` 0.05 _charactermovement))))

(event `InputAction|Run`
  (params (Key :type "Key Structure"))
  (bind _charactermovement (`Character.CharacterMovement` (`GameplayStatics.GetPlayerCharacter` 0)))
  ; Actions
  (:`Pressed`
    (`/Engine/EditorBlueprintResources/StandardMacros.FlipFlop`
      (:`A`
        (set `CharacterMovementComponent.MaxWalkSpeed` 1200.0 _charactermovement))
      (:`B`
        (set `CharacterMovementComponent.MaxWalkSpeed` 600.0 _charactermovement)))))

(event `InputAxis|moveleftright`
  (params (AxisValue :type "Float (single-precision)"))
  ; Movement
  (`self.AddMovementInput` (`KismetMathLibrary.GetRightVector` (`KismetMathLibrary.MakeRotator` 0.0 0.0 (.yaw (`self.GetControlRotation`)))) (* AxisValue (`self.SpeedModifier`)))
  (goto _label_3))

(event `InputAxis|rotateleftright`
  (params (AxisValue :type "Float (single-precision)"))
  ; Movement
  (`self.AddControllerYawInput` AxisValue))

(event `OnApexReached`
  (bind _charactermovement (`self.CharacterMovement`))
  ; For jump and double jump
  ;; For gliding
  (set `CharacterMovementComponent.GravityScale` 0.1 _charactermovement)
  (set `CharacterMovementComponent.AirControl` 0.8 _charactermovement))

(event `InputAxis|lookupdown`
  (params (AxisValue :type "Float (single-precision)"))
  ; Movement
  (`self.AddControllerPitchInput` AxisValue))

(event `self.K2_OnStartCrouch`
  (params (HalfHeightAdjust :type "Float (single-precision)") (ScaledHalfHeightAdjust :type "Float (single-precision)"))
  (bind _charactermovement (`self.CharacterMovement`))
  (bind _charactermovement_2 (`self.CharacterMovement`))
  ; Sliding
  (if (and (`self.shouldslideandcrounch`) (not (`self.is sliding`)))
    (set `self.is sliding` true)
    (set `self.shouldslideandcrounch` false)
    (set `self.crouch old friction` (`CharacterMovementComponent.GroundFriction` _charactermovement))
    (set `CharacterMovementComponent.GroundFriction` 0.0 _charactermovement)
    (set `self.old Max Walk Speed Crouched` (`CharacterMovementComponent.MaxWalkSpeedCrouched` _charactermovement_2))
    (set `CharacterMovementComponent.MaxWalkSpeedCrouched` 1500.0 _charactermovement_2)))

(event `start sliding`
  ; Sliding
  (set `self.shouldslideandcrounch` true)
  (`self.Crouch`))

(event `Key|Q`
  (params (Key :type "Key Structure"))
  (bind (_returnvalue _returnvalue2) (`self.wall trace macro` (`self.trace distance`)))
  (bind (_returnvalue_2 _returnvalue2_2) (`self.wall trace macro` (* (`self.trace distance`) -1)))
  ; wall running
  (:`Pressed`
    (if (`NavMovementComponent.IsFalling` (`self.CharacterMovement`))
      (`|ExecutionSequence`
        (:`then_0`
          (bind (_outhit _returnvalue_3) (`KismetSystemLibrary.SphereTraceSingle` _returnvalue _returnvalue2 20.0 "TraceTypeQuery1"))
          (if _returnvalue_3
            (set `self.wallslide` "NewEnumerator1")
            (`self.start wall run` :!label _label_4)
            (bind _returnvalue_4 (`KismetSystemLibrary.K2_SetTimerDelegate` (`|CreateDelegate` :!event `moveonthewall`) 0.01 true))
            (set `self.runtimer` _returnvalue_4)
            (`KismetSystemLibrary.Delay` (`self.runDuration`))
            (`self.stopwallrun` "MOVE_Falling")))
        (:`then_1`
          (bind (_outhit_2 _returnvalue_5) (`KismetSystemLibrary.SphereTraceSingle` _returnvalue_2 _returnvalue2_2 20.0 "TraceTypeQuery1"))
          (if _returnvalue_5
            (set `self.wallslide` "NewEnumerator0")
            (goto _label_4)))))))

(event `end sliding`
  ; Sliding
  (`self.UnCrouch`))

(event `Key|R`
  (params (Key :type "Key Structure"))
  ; Sliding
  (:`Pressed`
    (`self.start sliding`))
  (:`Released`
    (`self.end sliding`)))

(event `self.K2_OnEndCrouch`
  (params (HalfHeightAdjust :type "Float (single-precision)") (ScaledHalfHeightAdjust :type "Float (single-precision)"))
  (bind _charactermovement (`self.CharacterMovement`))
  ; Sliding
  (if (`self.is sliding`)
    (set `self.is sliding` false)
    (set `CharacterMovementComponent.GroundFriction` (`self.crouch old friction`) _charactermovement)
    (set `CharacterMovementComponent.MaxWalkSpeedCrouched` (`self.old Max Walk Speed Crouched`) _charactermovement)))

(event `start wall run`
  (bind _charactermovement (`self.CharacterMovement`))
  ; wall running
  (`CharacterMovementComponent.SetMovementMode` _charactermovement "MOVE_Flying" 0)
  (set `self.wallrunning` true)
  (set `CharacterMovementComponent.MaxFlySpeed` 1500.0 _charactermovement)
  (set `CharacterMovementComponent.MaxAcceleration` 10000.0 _charactermovement))

(event `moveonthewall`
  (bind (_returnvalue_x _returnvalue_y) (`KismetMathLibrary.BreakVector` (`KismetMathLibrary.Cross_VectorVector` (`self.wall trace Normal`) (`KismetMathLibrary.MakeVector` 0.0 0.0 (`KismetMathLibrary.SelectFloat` 1.0 -1.0 (`|EnumEquality` (`self.wallslide`) "NewEnumerator0"))))))
  (bind _returnvalue (+ (* (`self.GetActorForwardVector`) (* (`self.capsule radius`) 0.1)) (`self.K2_GetActorLocation`)))
  ; wall running
  (if (> (`KismetMathLibrary.VSize` (`self.GetVelocity`)) 0.5)
    (bind (_outhit _returnvalue_2) (`KismetSystemLibrary.SphereTraceSingle` :`Start` _returnvalue :`End` (+ _returnvalue (* (`self.GetActorRightVector`) (* (`self.capsule radius`) (`KismetMathLibrary.SelectFloat` -1.0 1.0 (`|EnumEquality` (`self.wallslide`) "NewEnumerator0"))))) :`Radius` (`self.capsule radius`) :`TraceChannel` "TraceTypeQuery1" :`DrawDebugType` "ForDuration"))
    (if _returnvalue_2
      (bind (_bblockinghit _binitialoverlap _time _distance _location _impactpoint _normal _impactnormal _physmat _hitactor _hitcomponent _hitbonename _bonename _hititem _elementindex _faceindex _tracestart) (`GameplayStatics.BreakHitResult` _outhit))
      (set `self.wall trace Normal` _impactnormal)
      (bind _output_get (set `self.distance to wall` (- (`KismetMathLibrary.VSize` (- _tracestart _impactpoint)) (`self.capsule radius`))))
      (`self.K2_AddActorWorldOffset` (* (`self.wall trace Normal`) (- _output_get 1.0)))
      (`self.AddMovementInput` (`KismetMathLibrary.MakeVector` _returnvalue_x _returnvalue_y (`KismetMathLibrary.SelectFloat` 0.0 0.0 (`self.arcrun`))))
      (else
        (`self.stopwallrun` "MOVE_Falling")))
    (else
      (`self.stopwallrun` "MOVE_Falling"))))

(fn `stopwallrun`
  (params (newmovementmode :type "EMovementMode Enum" :default "MOVE_None"))
  (bind _charactermovement (`self.CharacterMovement`))
  (`KismetSystemLibrary.K2_ClearAndInvalidateTimerHandle` (`self.runtimer`))
  (set `self.wallrunning` false)
  (set `CharacterMovementComponent.MaxFlySpeed` 600.0 _charactermovement)
  (set `CharacterMovementComponent.MaxAcceleration` 2048.0 _charactermovement)
  (`CharacterMovementComponent.SetMovementMode` _charactermovement newmovementmode 0))

(fn `UserConstructionScript`)